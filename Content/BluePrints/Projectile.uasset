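; Projectile actor that damages non-friendly targets it overlaps and plays impact effects.
; On overlap it checks for the IDamageable interface and the Friendly tag, then sends damage through EffectHealthMessage.
; Hostile hits and non-damageable overlaps both play an attached laser sound, spawn sparks and destroy the projectile.
; Friendly-tagged damageable actors are ignored, so the projectile does not react to them.
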(event Collision|EventActorBeginOverlap
  (params (OtherActor :type Actor%20Object%20Reference))
  (bind _returnvalue (Transformation|GetActorTransform))
  ;[1 1 1] Check if character is an enemy or a friendly character. (Though currently just to hit the enemy, Has future functionality if multiplayer was added to the game). Deals damage to the enemy, plays a hit sound and spawns a hit emmiter upon impact
  (if (Utilities|DoesObjectImplementInterface OtherActor "/Game/BluePrints/IDamageable.IDamageable_C")
    (if (not (Actor|ActorHasTag OtherActor "Friendly"))
      (Class|IDamageable|EffectHealth(Message) OtherActor (Variables|Default|GetDamage))
      (bind _returnvalue_2 (Audio|SpawnSoundAttached "/Game/Audio/SoundsCrate-SciFi-Laser5.SoundsCrate-SciFi-Laser5" (Variables|Default|GetProjectileCollision) :!label _label))
      (Audio|Components|Audio|AdjustVolume _returnvalue_2 0.0 0.45 :!class /Script/Engine.AudioComponent)
      (Effects|SpawnEmitteratLocation "/Game/StarterContent/Particles/LaserSparks.LaserSparks" (.location _returnvalue) (.rotation _returnvalue))
      (Actor|DestroyActor))
    (else
      (goto _label))))

(fn ConstructionScript)