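; Enemy character Blueprint that takes damage, awards score on death and hurts the hero on contact.
; EffectHealth recalculates health; when dead it removes the damage volume, adds to the TwinStickMode score, ignores pawn and world collision, detaches its controller, then spawns an explosion and destroys itself after a brief delay.
; Overlapping the hero starts a looping timer that applies damage at the attacks-per-second rate until the overlap ends.
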(event Custom|DamageTheHero
  ;[1 1 1] Damage Hero Character - Sets rate of attacks as well as damage towards the player
  (Default|EffectHealth (Variables|Default|GetHero) (Variables|Default|GetDamage)))

(event Collision|EventActorBeginOverlap
  (params (OtherActor :type Actor%20Object%20Reference))
  ;[1 1 1] Damage Hero Character - Sets rate of attacks as well as damage towards the player
  (bind _ashero_character (Utilities|Casting|CastToHeroCharacter OtherActor))
  (Variables|Default|SetHero _ashero_character)
  (Utilities|Time|SetTimerbyFunctionName 0 "DamageTheHero" (/ 1.0 (Variables|Default|GetAttacksPerSecond)) true))

(event Collision|EventActorEndOverlap
  (params (OtherActor :type Actor%20Object%20Reference))
  ;[1 1 1] Damage Hero Character - Sets rate of attacks as well as damage towards the player
  (if (== OtherActor (Variables|Default|GetHero))
    (Utilities|Time|ClearTimerbyFunctionName 0 "DamageTheHero")))

(event EventEffectHealth
  (params (Delta :type Float%20%28single-precision%29))
  (bind _capsulecomponent (Variables|Default|GetCapsuleComponent))
  ;[1 1 1] Enemy Health and Death - Sets Enemy health and checks for when the Enemy is dead. Upon death, Destroys Damage Volume, Turns of collision  and Adds to the Score Value before exsploding a few moments later.
  (Class|BaseCharacter|CalculateHealth Delta)
  (if (Variables|Default|GetisDead)
    (Components|DestroyComponent (Variables|Default|GetDamageVolume))
    (bind _astwin_stick_mode (Utilities|Casting|CastToTwinStickMode (Game|GetGameMode)))
    (Default|IncrementScore _astwin_stick_mode (Variables|Default|GetScore))
    (Collision|SetCollisionResponsetoChannel _capsulecomponent "ECC_WorldDynamic" "ECR_Ignore")
    (Collision|SetCollisionResponsetoChannel _capsulecomponent "ECC_Pawn" "ECR_Ignore")
    (Class|Pawn|DetachfromControllerPendingDestroy)
    (Utilities|FlowControl|Delay 0.1)
    (Game|SpawnActorfromClass "/Game/BluePrints/Explosion.Explosion_C" (Transformation|GetActorTransform) "Undefined" 0 0)
    (Actor|DestroyActor)))

(fn ConstructionScript)