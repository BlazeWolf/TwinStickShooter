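; Weapon Blueprint for an automatic gun that fires projectiles for as long as the trigger is held.
; PullTrigger passes a DoOnce gate, fires immediately and starts a looping timer on Fire at an interval derived from RoundsPerSecond.
; Each Fire plays a quietened sci-fi laser sound attached to the gun mesh and spawns a projectile at the spawn point.
; ReleaseTrigger clears the timer and resets the gate.
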(event Custom|PullTrigger
  ;[1 1 1] Gun Firing
  (Utilities|FlowControl|DoOnce false
    (:Completed
      (CallFunction|Fire)
      (Utilities|Time|SetTimerbyFunctionName 0 "Fire" (/ 1.0 (Variables|Default|GetRoundsPerSecond)) true))))

(event Custom|ReleaseTrigger
  ;[1 1 1] Gun Firing
  (Utilities|Time|ClearTimerbyFunctionName 0 "Fire")
  (Utilities|FlowControl|DoOnce false) ; enters at Reset
)

(event Custom|Fire
  ;[1 1 1] Gun Firing
  (bind _returnvalue (Audio|SpawnSoundAttached "/Game/Audio/SoundsCrate-SciFi-Laser1.SoundsCrate-SciFi-Laser1" (Variables|Default|GetGunMesh)))
  (Audio|Components|Audio|AdjustVolume _returnvalue 0.0 0.15 :!class /Script/Engine.AudioComponent)
  (Game|SpawnActorfromClass "/Game/BluePrints/Projectile.Projectile_C" (Transformation|GetWorldTransform (Variables|Default|GetProjectileSpawnPoint)) "Undefined" 0 0))

(fn ConstructionScript)