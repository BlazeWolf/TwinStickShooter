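; HeroCharacter is the twin-stick shooter player character, handling movement, aiming, health, death and respawn.
; BeginPlay spawns a weapon on GunSocket, records the spawn transform in TwinStickMode and adds the HUD.
; Move axes drive world-space movement, while look axes past a deadzone set control rotation and pull the weapon trigger, releasing it otherwise.
; EffectHealth updates health and, on death, disables input, waits, requests a GameMode respawn, then destroys weapon and character.
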(event EventBeginPlay
  (bind _mesh (Variables|Character|GetMesh))
  ;[1 1 1] Spawning - Spawns Player at "Player Start", Spawn weapon (Attached to the Player and set to a world transform) and Activates the play HUD
  (Utilities|FlowControl|Sequence
    (:then_0
      (bind _returnvalue (Game|SpawnActorfromClass "/Game/BluePrints/Weapon.Weapon_C" (Transformation|GetWorldTransform _mesh) "Undefined" 0 0))
      (bind _output_get (Variables|Default|SetWeapon _returnvalue))
      (Transformation|AttachComponentToComponent _output_get _mesh "GunSocket" "SnapToTarget" "SnapToTarget" "KeepWorld" true))
    (:then_1
      (bind _astwin_stick_mode (Utilities|Casting|CastToTwinStickMode (Game|GetGameMode)))
      (bind _output_get_2 (Variables|Default|SetGame%20Mode _astwin_stick_mode))
      (Variables|/Game/BluePrints/TwinStickMode.TwinStickMode_C|SetPlayerSpawnTransform _output_get_2 (Transformation|GetActorTransform)))
    (:then_2
      (bind _returnvalue_2 (UserInterface|CreateWidget "/Game/BluePrints/TwinStickHud.TwinStickHud_C"))
      (UserInterface|Viewport|AddtoViewport _returnvalue_2 0))))

(event EventEffectHealth
  (params (Delta :type Float%20%28single-precision%29))
  ;[1 1 1] HeroCharacter Health / Death / Respawn - Sets player health, Checks for if the player is dead, Upon death disables Input, Destroys the Actor and Respawns the player at player start
  (Class|BaseCharacter|CalculateHealth Delta)
  (if (Variables|Default|GetisDead)
    (Input|DisableInput 0)
    (Utilities|FlowControl|Delay 3.0)
    (Default|RespawnPlayer (Variables|Default|GetGame%20Mode))
    (Actor|DestroyActor (Variables|Default|GetWeapon))))

(event Input|AxisEvents|InputAxisMoveUp
  (params (AxisValue :type Float%20%28single-precision%29))
  ;[1 1 1] Movement
  (Pawn|Input|AddMovementInput "1.000000, 0, 0" AxisValue false))

(event Input|AxisEvents|InputAxisMoveRight
  (params (AxisValue :type Float%20%28single-precision%29))
  ;[1 1 1] Movement
  (Pawn|Input|AddMovementInput "0.000000,1.000000, 0" AxisValue false))

(event Input|AxisEvents|InputAxisLookUp
  (params (AxisValue :type Float%20%28single-precision%29))
  (bind _weapon (Variables|Default|GetWeapon))
  ;[1 1 1] Rotation
  (if (> (Math|Vector|VectorLength (Math|Vector|MakeVector AxisValue (stale Input|AxisEvents|InputAxisLookRight AxisValue) 0.0)) 0.25)
    (Pawn|SetControlRotation (Pawn|GetController) (Math|Conversions|RotationFromXVector (Math|Vector|MakeVector AxisValue (stale Input|AxisEvents|InputAxisLookRight AxisValue) 0.0)))
    ;[1 1 1] Firing on rotation
    (Default|PullTrigger _weapon)
    (else
      (Default|ReleaseTrigger _weapon))))

(event Input|AxisEvents|InputAxisLookRight
  (params (AxisValue :type Float%20%28single-precision%29))
  (bind _weapon (Variables|Default|GetWeapon))
  ;[1 1 1] Rotation
  (if (> (Math|Vector|VectorLength (Math|Vector|MakeVector (stale Input|AxisEvents|InputAxisLookUp AxisValue) AxisValue 0.0)) 0.25)
    (Pawn|SetControlRotation (Pawn|GetController) (Math|Conversions|RotationFromXVector (Math|Vector|MakeVector (stale Input|AxisEvents|InputAxisLookUp AxisValue) AxisValue 0.0)))
    ;[1 1 1] Firing on rotation
    (Default|PullTrigger _weapon)
    (else
      (Default|ReleaseTrigger _weapon))))

(fn ConstructionScript)